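; Player controller for a two-team multiplayer game that spawns and possesses the Hero pawn and updates team scores.
; RespawnHero spawns at a PlayerStart picked by array index, then caches the team from MyPlayerState.
; BeginPlay spawns at index 0 on authority, while CheckRespawnHero maps the GameInstance team to index 0 or 1.
; CoreTeam increments the opposing team's Core counter in MyGameState.
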(event Custom|RespawnHero
  (params (Dimension%201 :type Integer))
  (bind _outactors (Actor|GetAllActorsOfClass "/Script/Engine.PlayerStart"))
  (bind _returnvalue (Game|SpawnActorfromClass "/Game/GameMultiplayer/Character/Hero.Hero_C" (Transformation|GetActorTransform (Utilities|Array|Get(acopy) _outactors Dimension%201)) "Undefined" self 0))
  (Pawn|Possess self _returnvalue)
  (bind _asmy_player_state (Utilities|Casting|CastToMyPlayerState (Variables|GetPlayerState)))
  (Variables|Default|SetStateTeam (Variables|/Game/GameMultiplayer/Blueprints/MyPlayerState.MyPlayerState_C|GetTeam%20red%20or%20Blue _asmy_player_state)))

(event Custom|CoreTeam
  (bind _asmy_game_state (Utilities|Casting|CastToMyGameState (Game|GetGameState)))
  (switch Utilities|FlowControl|Switch|SwitchonRedOrBlue (Variables|Default|GetStateTeam)
    (:NewEnumerator0
      (Variables|/Game/GameMultiplayer/Blueprints/MyGameState.MyGameState_C|SetCoreBlue _asmy_game_state (+ (Variables|/Game/GameMultiplayer/Blueprints/MyGameState.MyGameState_C|GetCoreBlue _asmy_game_state) 1)))
    (:NewEnumerator1
      (Variables|/Game/GameMultiplayer/Blueprints/MyGameState.MyGameState_C|SetCoreRed _asmy_game_state (+ (Variables|/Game/GameMultiplayer/Blueprints/MyGameState.MyGameState_C|GetCoreRed _asmy_game_state) 1)))))

(event Custom|CheckRespawnHero
  (bind _asmy_game_instance (Utilities|Casting|CastToMyGameInstance (Game|GetGameInstance)))
  (switch Utilities|FlowControl|Switch|SwitchonRedOrBlue (Variables|/Game/GameMultiplayer/Blueprints/MyGameInstance.MyGameInstance_C|GetTeamRedOrBlue _asmy_game_instance)
    (:NewEnumerator0
      (CallFunction|RespawnHero))
    (:NewEnumerator1
      (CallFunction|RespawnHero 1))))

(event EventBeginPlay
  (Networking|SwitchHasAuthority
    (:Authority
      (CallFunction|RespawnHero self (Class|KismetMathLibrary|SignOfInteger)))))

(fn ConstructionScript)